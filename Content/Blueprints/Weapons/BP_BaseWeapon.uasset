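; BP_BaseWeapon is a weapon base with empty shoot and stop events, plus shared firing, sound and ammo logic.
; Fireweapon line-traces to apply damage, spawning blood on enemy-tagged actors, while Fireprojectile spawns a projectile with the weapon's damage and speed.
; Ammo checks and decrements switch on Ammotype, using counts stored on the cached first-person player character and refreshing its HUD after each decrement.
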(event Custom|Play%20weapon%20sound
  ;[1 1 1] Play weapon sound
  (Audio|PlaySoundatLocation (Variables|Settings|GetSound) (Transformation|GetActorLocation) "0, 0, 0" 1.0 1.0 0.0 0 0 0 0))

(event Custom|ShootWeapon)

(event Custom|StopShooting)

(event Custom|Decreaseammo
  (bind _playercharacterref (Variables|Settings|Getplayercharacterref))
  (bind _playercharacterref_2 (Variables|Settings|Getplayercharacterref))
  (bind _playercharacterref_3 (Variables|Settings|Getplayercharacterref))
  (bind _playercharacterref_4 (Variables|Settings|Getplayercharacterref))
  ;[1 1 1] Decrease ammo
  (switch Utilities|FlowControl|Switch|SwitchonAmmo (Variables|Settings|Getammotype)
    (:NewEnumerator0
      (Math|Integer|DecrementInt (Variables|/Game/FirstPerson/Blueprints/BP_FirstPersonCharacter.BP_FirstPersonCharacter_C|Getbullet _playercharacterref_2)
        (:%20%20
          (Default|Updatebulletammo (Variables|/Game/FirstPerson/Blueprints/BP_FirstPersonCharacter.BP_FirstPersonCharacter_C|GetPlayerhud _playercharacterref_2)))))
    (:NewEnumerator1
      (Math|Integer|DecrementInt (Variables|/Game/FirstPerson/Blueprints/BP_FirstPersonCharacter.BP_FirstPersonCharacter_C|Getshell _playercharacterref_3)
        (:%20%20
          (Default|Updateshellammo (Variables|/Game/FirstPerson/Blueprints/BP_FirstPersonCharacter.BP_FirstPersonCharacter_C|GetPlayerhud _playercharacterref_3)))))
    (:NewEnumerator2
      (Math|Integer|DecrementInt (Variables|/Game/FirstPerson/Blueprints/BP_FirstPersonCharacter.BP_FirstPersonCharacter_C|Getrock _playercharacterref_4)
        (:%20%20
          (Default|Updaterocketammo (Variables|/Game/FirstPerson/Blueprints/BP_FirstPersonCharacter.BP_FirstPersonCharacter_C|GetPlayerhud _playercharacterref_4)))))
    (:NewEnumerator3
      (Math|Integer|DecrementInt (Variables|/Game/FirstPerson/Blueprints/BP_FirstPersonCharacter.BP_FirstPersonCharacter_C|Getcell _playercharacterref)
        (:%20%20
          (Default|Updatecellammo (Variables|/Game/FirstPerson/Blueprints/BP_FirstPersonCharacter.BP_FirstPersonCharacter_C|GetPlayerhud _playercharacterref)))))))

(event EventBeginPlay
  (bind _asbp_first_person_character (Utilities|Casting|CastToBP_FirstPersonCharacter (Game|GetPlayerCharacter 0)))
  (Variables|Settings|Setplayercharacterref _asbp_first_person_character))

(fn ConstructionScript)

(fn Fireweapon
  (bind _linetrace (Variables|Default|Getlinetrace))
  (bind _returnvalue (Transformation|GetWorldLocation _linetrace))
  (bind (_outhit _returnvalue_2) (Collision|LineTraceForObjects _returnvalue (+ _returnvalue (* (Math|Vector|GetForwardVector (Transformation|GetWorldRotation (Variables|Default|Getlinetrace))) (Variables|Settings|Getlinetracedistance))) (Utilities|Array|MakeArray "ObjectTypeQuery1" "ObjectTypeQuery2" "ObjectTypeQuery3") false (Utilities|Array|MakeArray self (Game|GetPlayerCharacter 0)) "None"))
  (if _returnvalue_2
    (Game|Damage|ApplyDamage (.HitActor (Collision|BreakHitResult _outhit)) (Variables|Settings|Getweapondamage) 0 0)
    (if (Actor|ActorHasTag (.HitActor (Collision|BreakHitResult _outhit)) "enemy")
      (Game|SpawnActorfromClass "/Game/Blueprints/Blood/BP_Blood.BP_Blood_C" (Math|Transform|MakeTransform (.Location (Collision|BreakHitResult _outhit)) (Math|Rotator|MakeRotfromY (.Normal (Collision|BreakHitResult _outhit))) "1.000000,1.000000,1.000000") "Undefined" 0 0))))

(fn Hasenoughammo?
  (switch Utilities|FlowControl|Switch|SwitchonAmmo (Variables|Settings|Getammotype)
    (:NewEnumerator0
      (if (> (Variables|/Game/FirstPerson/Blueprints/BP_FirstPersonCharacter.BP_FirstPersonCharacter_C|Getbullet (Variables|Settings|Getplayercharacterref)) 0)
        (return true)
        (else
          (return false))))
    (:NewEnumerator1
      (if (> (Variables|/Game/FirstPerson/Blueprints/BP_FirstPersonCharacter.BP_FirstPersonCharacter_C|Getshell (Variables|Settings|Getplayercharacterref)) 0)
        (return true)
        (else
          (return false))))
    (:NewEnumerator2
      (if (> (Variables|/Game/FirstPerson/Blueprints/BP_FirstPersonCharacter.BP_FirstPersonCharacter_C|Getrock (Variables|Settings|Getplayercharacterref)) 0)
        (return true)
        (else
          (return false))))
    (:NewEnumerator3
      (if (> (Variables|/Game/FirstPerson/Blueprints/BP_FirstPersonCharacter.BP_FirstPersonCharacter_C|Getcell (Variables|Settings|Getplayercharacterref)) 0)
        (return true)
        (else
          (return false))))))

(fn Fireprojectile
  (Game|SpawnActorfromClass (Variables|Settings|GetProjectile) (Transformation|GetWorldTransform (Variables|Default|Getprojectilescene)) "Undefined" 0 (Variables|Settings|GetProjectilespeed) (Variables|Settings|Getweapondamage) 0))