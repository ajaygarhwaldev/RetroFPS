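; BFG weapon Blueprint that fires a projectile at a cost of cell ammo from the player character.
; ShootWeapon checks for enough cells, then a DoOnce gate blocks refiring while the sound and fire flipbook play.
; After a delay matching the flipbook length, it fires, returns to idle, deducts ammo, updates the HUD and resets the gate.
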(event Custom|RESETDOONCE
  (bind _playercharacterref (Variables|Default|Getplayercharacterref))
  (bind _weaponflipbook (Variables|Default|GetWeaponflipbook))
  (Utilities|FlowControl|DoOnce false) ; enters at Reset
)

(event EventShootWeapon
  (bind _playercharacterref (Variables|Default|Getplayercharacterref))
  (bind _weaponflipbook (Variables|Default|GetWeaponflipbook))
  (if (>= (Variables|/Game/FirstPerson/Blueprints/BP_FirstPersonCharacter.BP_FirstPersonCharacter_C|Getcell (Variables|Default|Getplayercharacterref)) 30)
    (Utilities|FlowControl|DoOnce false
      (:Completed
        (CallFunction|PlayWeaponSound)
        (Sprite|SetFlipbook _weaponflipbook "/Game/Sprites/Weapons/BFG/BFGFire.BFGFire")
        (Utilities|FlowControl|Delay (Class|PaperFlipbookComponent|GetFlipbookLength _weaponflipbook))
        (CallFunction|Fireprojectile)
        (Sprite|SetFlipbook (Variables|Default|GetWeaponflipbook) "/Game/Sprites/Weapons/BFG/BFGIdle.BFGIdle")
        (Variables|/Game/FirstPerson/Blueprints/BP_FirstPersonCharacter.BP_FirstPersonCharacter_C|Setcell _playercharacterref (- (Variables|/Game/FirstPerson/Blueprints/BP_FirstPersonCharacter.BP_FirstPersonCharacter_C|Getcell _playercharacterref) 30))
        (Default|Updatecellammo (Variables|/Game/FirstPerson/Blueprints/BP_FirstPersonCharacter.BP_FirstPersonCharacter_C|GetPlayerhud _playercharacterref))
        (CallFunction|RESETDOONCE)))))

(fn ConstructionScript
  (|CallParentFunction))