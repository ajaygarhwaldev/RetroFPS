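; BP_Chainsaw is a chainsaw weapon that attacks repeatedly while shooting is active.
; ShootWeapon passes through a DoOnce to start a short looping timer, which prevents duplicate timers from repeated calls.
; Each timer tick calls Fireweapon, plays the weapon sound and sets the active flipbook.
; StopShooting clears the timer, restores the idle flipbook and resets the DoOnce.
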(event Custom|Usechainsaw
  (CallFunction|Fireweapon)
  (CallFunction|PlayWeaponSound)
  (Sprite|SetFlipbook (Variables|Default|GetWeaponflipbook) "/Game/Sprites/Weapons/Chainsaw/Chainsawactive.Chainsawactive"))

(event Custom|resetchainsaw
  (Utilities|FlowControl|DoOnce false) ; enters at Reset
)

(event EventBeginPlay
  (|CallParentFunction) ; This node is disabled and will not be called.\nDrag off pins to build functionality.
)

(event Collision|EventActorBeginOverlap
  (params (OtherActor :type Actor%20Object%20Reference))
  (|CallParentFunction OtherActor) ; This node is disabled and will not be called.\nDrag off pins to build functionality.
)

(event EventTick
  (params (DeltaSeconds :type Float%20%28single-precision%29))
  (|CallParentFunction DeltaSeconds) ; This node is disabled and will not be called.\nDrag off pins to build functionality.
)

(event EventShootWeapon
  (Utilities|FlowControl|DoOnce false
    (:Completed
      (bind _returnvalue (Utilities|Time|SetTimerbyEvent (delegate Custom|Usechainsaw) 0.15 true))
      (Variables|Default|Setchainsawevent _returnvalue))))

(event EventStopShooting
  (Utilities|Time|ClearandInvalidateTimerbyHandle (Variables|Default|Getchainsawevent))
  (Sprite|SetFlipbook (Variables|Default|GetWeaponflipbook) "/Game/Sprites/Weapons/Chainsaw/Chainsawidle.Chainsawidle")
  (CallFunction|Resetchainsaw))

(fn ConstructionScript
  (|CallParentFunction))