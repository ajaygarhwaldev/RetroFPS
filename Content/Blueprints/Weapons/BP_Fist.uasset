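; BP_Fist is a melee fist weapon that plays a flipbook punch when the player attacks.
; ShootWeapon passes through a DoOnce gate, calls Fireweapon, which is not defined in this graph, and switches the weapon flipbook to the punch animation.
; A delay matching the flipbook's length then restores the idle flipbook and calls Resetattack to reopen the gate, so punches cannot overlap.
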(event Custom|resetattack
  (bind _weaponflipbook (Variables|Default|GetWeaponflipbook))
  (Utilities|FlowControl|DoOnce false) ; enters at Reset
)

(event EventBeginPlay
  (|CallParentFunction) ; This node is disabled and will not be called.\nDrag off pins to build functionality.
)

(event Collision|EventActorBeginOverlap
  (params (OtherActor :type Actor%20Object%20Reference))
  (|CallParentFunction OtherActor) ; This node is disabled and will not be called.\nDrag off pins to build functionality.
)

(event EventTick
  (params (DeltaSeconds :type Float%20%28single-precision%29))
  (|CallParentFunction DeltaSeconds) ; This node is disabled and will not be called.\nDrag off pins to build functionality.
)

(event EventShootWeapon
  (bind _weaponflipbook (Variables|Default|GetWeaponflipbook))
  (Utilities|FlowControl|DoOnce false
    (:Completed
      (CallFunction|Fireweapon)
      (Sprite|SetFlipbook _weaponflipbook "/Game/Sprites/Weapons/Punch/Punchattack.Punchattack")
      (Utilities|FlowControl|Delay (Class|PaperFlipbookComponent|GetFlipbookLength _weaponflipbook))
      (Sprite|SetFlipbook (Variables|Default|GetWeaponflipbook) "/Game/Sprites/Weapons/Punch/Punchidle.Punchidle")
      (CallFunction|Resetattack))))

(fn ConstructionScript
  (|CallParentFunction))