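; BP_Placeditem is a placed world item shown as a 2D Paper sprite that always turns to face the player.
; The construction script applies an exposed sprite and scale to the PaperSprite component.
; On Tick, it sets its yaw toward the first player character with a look-at rotation, acting as a vertical-axis billboard.
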(event EventTick
  (params (DeltaSeconds :type Float%20%28single-precision%29))
  ;[1 1 1] Face player
  (Transformation|SetActorRotation (Math|Rotator|MakeRotator 0.0 0.0 (.yaw (Math|Rotator|FindLookatRotation (Transformation|GetActorLocation) (Transformation|GetActorLocation (Game|GetPlayerCharacter 0)))))))

(fn ConstructionScript
  (Rendering|Components|Sprite|SetSprite (Variables|Default|GetPaperSprite) (Variables|Default|GetNew%20Sprite))
  (Transformation|SetWorldScale3D (Variables|Default|GetPaperSprite) (Variables|Default|GetNew%20Scale)))