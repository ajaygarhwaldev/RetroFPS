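; Ammo pickup that gives the player bullets, shells, rockets or cells, depending on its Ammotype.
; The construction script sets the Paper2D sprite from that type, and Tick yaws the actor toward the player like a billboard.
; When BP_FirstPersonCharacter overlaps the box, a DoOnce adds the configured amount to the matching count, clamped to its maximum, refreshes that HUD readout and destroys the pickup.
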(event OnComponentBeginOverlap(Box)
  (params (OverlappedComponent :type Primitive%20Component%20Object%20Reference) (OtherActor :type Actor%20Object%20Reference) (OtherComp :type Primitive%20Component%20Object%20Reference) (OtherBodyIndex :type Integer) (bFromSweep :type Boolean) (SweepResult :type Hit%20Result%20Structure%20%28by%20ref%29))
  ;[1 1 1] Give player ammo when they overlap the box
  (bind _asbp_first_person_character (Utilities|Casting|CastToBP_FirstPersonCharacter OtherActor))
  (Variables|Default|SetAs%20BP%20First%20Person%20Character _asbp_first_person_character)
  (Utilities|FlowControl|DoOnce false
    (:Completed
      (switch Utilities|FlowControl|Switch|SwitchonAmmotype (Variables|Default|Getammotype)
        (:NewEnumerator0
          (Variables|/Game/FirstPerson/Blueprints/BP_FirstPersonCharacter.BP_FirstPersonCharacter_C|Setbullet (Variables|Default|GetAs%20BP%20First%20Person%20Character) (Math|Integer|Clamp(Integer) (+ (Variables|/Game/FirstPerson/Blueprints/BP_FirstPersonCharacter.BP_FirstPersonCharacter_C|Getbullet (Variables|Default|GetAs%20BP%20First%20Person%20Character)) (Variables|Default|Gethowmuchammotigiveplayer)) 0 (Variables|/Game/FirstPerson/Blueprints/BP_FirstPersonCharacter.BP_FirstPersonCharacter_C|Getmaxbullet (Variables|Default|GetAs%20BP%20First%20Person%20Character))))
          (Default|Updatebulletammo (Variables|/Game/FirstPerson/Blueprints/BP_FirstPersonCharacter.BP_FirstPersonCharacter_C|GetPlayerhud (Variables|Default|GetAs%20BP%20First%20Person%20Character)))
          (Actor|DestroyActor))
        (:NewEnumerator1
          (Variables|/Game/FirstPerson/Blueprints/BP_FirstPersonCharacter.BP_FirstPersonCharacter_C|Setshell (Variables|Default|GetAs%20BP%20First%20Person%20Character) (Math|Integer|Clamp(Integer) (+ (Variables|/Game/FirstPerson/Blueprints/BP_FirstPersonCharacter.BP_FirstPersonCharacter_C|Getshell (Variables|Default|GetAs%20BP%20First%20Person%20Character)) (Variables|Default|Gethowmuchammotigiveplayer)) 0 (Variables|/Game/FirstPerson/Blueprints/BP_FirstPersonCharacter.BP_FirstPersonCharacter_C|Getmaxshell (Variables|Default|GetAs%20BP%20First%20Person%20Character))))
          (Default|Updateshellammo (Variables|/Game/FirstPerson/Blueprints/BP_FirstPersonCharacter.BP_FirstPersonCharacter_C|GetPlayerhud (Variables|Default|GetAs%20BP%20First%20Person%20Character)))
          (Actor|DestroyActor))
        (:NewEnumerator2
          (Variables|/Game/FirstPerson/Blueprints/BP_FirstPersonCharacter.BP_FirstPersonCharacter_C|Setrock (Variables|Default|GetAs%20BP%20First%20Person%20Character) (Math|Integer|Clamp(Integer) (+ (Variables|/Game/FirstPerson/Blueprints/BP_FirstPersonCharacter.BP_FirstPersonCharacter_C|Getrock (Variables|Default|GetAs%20BP%20First%20Person%20Character)) (Variables|Default|Gethowmuchammotigiveplayer)) 0 (Variables|/Game/FirstPerson/Blueprints/BP_FirstPersonCharacter.BP_FirstPersonCharacter_C|Getmaxrock (Variables|Default|GetAs%20BP%20First%20Person%20Character))))
          (Default|Updaterocketammo (Variables|/Game/FirstPerson/Blueprints/BP_FirstPersonCharacter.BP_FirstPersonCharacter_C|GetPlayerhud (Variables|Default|GetAs%20BP%20First%20Person%20Character)))
          (Actor|DestroyActor))
        (:NewEnumerator3
          (Variables|/Game/FirstPerson/Blueprints/BP_FirstPersonCharacter.BP_FirstPersonCharacter_C|Setcell (Variables|Default|GetAs%20BP%20First%20Person%20Character) (Math|Integer|Clamp(Integer) (+ (Variables|/Game/FirstPerson/Blueprints/BP_FirstPersonCharacter.BP_FirstPersonCharacter_C|Getcell (Variables|Default|GetAs%20BP%20First%20Person%20Character)) (Variables|Default|Gethowmuchammotigiveplayer)) 0 (Variables|/Game/FirstPerson/Blueprints/BP_FirstPersonCharacter.BP_FirstPersonCharacter_C|Getmaxcell (Variables|Default|GetAs%20BP%20First%20Person%20Character))))
          (Default|Updatecellammo (Variables|/Game/FirstPerson/Blueprints/BP_FirstPersonCharacter.BP_FirstPersonCharacter_C|GetPlayerhud (Variables|Default|GetAs%20BP%20First%20Person%20Character)))
          (Actor|DestroyActor))))))

(event EventTick
  (params (DeltaSeconds :type Float%20%28single-precision%29))
  ;[1 1 1] Face Player
  (Transformation|SetActorRotation (Math|Rotator|MakeRotator 0.0 0.0 (.yaw (Math|Rotator|FindLookatRotation (Transformation|GetActorLocation) (Transformation|GetActorLocation (Game|GetPlayerCharacter 0)))))))

(fn ConstructionScript
  (switch Utilities|FlowControl|Switch|SwitchonAmmotype (Variables|Default|Getammotype)
    (:NewEnumerator0
      (Rendering|Components|Sprite|SetSprite (Variables|Default|GetPaperSprite) "/Game/Sprites/Items/NormalAmmo_Sprite.NormalAmmo_Sprite"))
    (:NewEnumerator1
      (Rendering|Components|Sprite|SetSprite (Variables|Default|GetPaperSprite) "/Game/Sprites/Items/Shotgun_Sprite.Shotgun_Sprite"))
    (:NewEnumerator2
      (Rendering|Components|Sprite|SetSprite (Variables|Default|GetPaperSprite) "/Game/Sprites/Items/Rocket_Sprite.Rocket_Sprite"))
    (:NewEnumerator3
      (Rendering|Components|Sprite|SetSprite (Variables|Default|GetPaperSprite) "/Game/Sprites/Items/cellammo_Sprite.cellammo_Sprite"))))