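; Explosive barrel item, drawn as a Paper2D flipbook, that blows up when it takes any damage.
; Every tick it yaws toward the player character, billboard-style.
; On damage it switches to the explosion flipbook and applies barrel damage to pawn hits from a sphere trace around itself.
; It destroys itself once the flipbook's length has elapsed.
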(event EventTick
  (params (DeltaSeconds :type Float%20%28single-precision%29))
  ;[1 1 1] Face player character
  (Transformation|SetActorRotation (Math|Rotator|MakeRotator 0.0 0.0 (.yaw (Math|Rotator|FindLookatRotation (Transformation|GetActorLocation) (Transformation|GetActorLocation (Game|GetPlayerCharacter 0)))))))

(event Game|Damage|EventAnyDamage
  (params (Damage :type Float%20%28single-precision%29) (DamageType :type Damage%20Type%20Object%20Reference) (InstigatedBy :type Controller%20Object%20Reference) (DamageCauser :type Actor%20Object%20Reference))
  (bind _returnvalue (Transformation|GetActorLocation))
  ;[1 1 1] Explode barrel when it is damaged
  (Sprite|SetFlipbook (Variables|Default|GetPaperFlipbook) "/Game/Sprites/Projectiles/Rocket/rocketexplosion.rocketexplosion")
  (bind _outhits (Collision|MultiSphereTraceForObjects _returnvalue _returnvalue 4.5e+02 (Utilities|Array|MakeArray "ObjectTypeQuery3") false 0 "None"))
  (for _array_element _outhits
    (Game|Damage|ApplyDamage (.HitActor (Collision|BreakHitResult _array_element)) (Variables|Default|Getbarreldamage) 0 0))
  (Utilities|FlowControl|Delay (Class|PaperFlipbookComponent|GetFlipbookLength (Variables|Default|GetPaperFlipbook)))
  (Actor|DestroyActor))

(fn ConstructionScript)