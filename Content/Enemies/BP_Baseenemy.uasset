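; Base enemy character drawn as a Doom-style directional sprite, with health, melee and projectile attacks, and death animation.
; Pawn sensing of the player, or non-lethal damage, sets the canseeplayer blackboard key; sight clears it after a retriggerable delay.
; Each tick derives idle, moving or attack state and uses dot-product viewing angle to pick flipbook and rotation.
; Death stops AI logic and collision, then destroys the actor; rotate-towards-player is an empty event.
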(event OnSeePawn(PawnSensing)
  (params (Pawn :type Pawn%20Object%20Reference))
  ;[1 1 1] Handle enemy vision
  (Utilities|Casting|CastToBP_FirstPersonCharacter Pawn)
  (Variables|donotedit|Setcanseeplayer true)
  (AI|Components|Blackboard|SetValueasBool (AI|GetBlackboard 0) (Utilities|Name|MakeLiteralName "canseeplayer") true)
  (Utilities|FlowControl|RetriggerableDelay 0.7)
  (Variables|donotedit|Setcanseeplayer false)
  (AI|Components|Blackboard|SetValueasBool (AI|GetBlackboard 0) (Utilities|Name|MakeLiteralName "canseeplayer") false))

(event OnHearNoise(PawnSensing)
  (params (Instigator :type Pawn%20Object%20Reference) (Location :type Vector%20%28by%20ref%29 :default "0, 0, 0") (Volume :type Float%20%28single-precision%29))
  ;[1 1 1] handle enemy damage
  (if (== Instigator (Game|GetPlayerCharacter 0))
    (Variables|donotedit|Setcanseeplayer true)
    (AI|Components|Blackboard|SetValueasBool (AI|GetBlackboard 0) (Utilities|Name|MakeLiteralName "canseeplayer") true)))

(event Custom|Rotatetowardsplayer
  ;[1 1 1] handle enemy rotation
)

(event Custom|SpawnProjectile
  ;[1 1 1] Attack system
  ;;[1 0 0] ranged attack
  (Variables|Donotedit|Setisattacking true)
  (Variables|Donotedit|Setattackstate "NewEnumerator3")
  (Components|Movement|StopMovementImmediately (Variables|Character|GetCharacterMovement))
  (Game|SpawnActorfromClass (Variables|Edit|Getenemyprojectile) (Transformation|GetWorldTransform (Variables|Default|Getprojectilespawn)) "Undefined" 0 (Variables|Edit|GetProjectilespeed) (Variables|Edit|GetProjectiledamage) 0)
  (Utilities|FlowControl|RetriggerableDelay (+ (Variables|Edit|GetFirerate) 0.3))
  (Variables|Donotedit|Setisattacking false))

(event Custom|Meleeattack
  (bind _returnvalue (Transformation|GetActorLocation))
  ;[1 1 1] Attack system
  ;;[1 0 0] melee attack
  (Variables|Donotedit|Setisattacking true)
  (Variables|Donotedit|Setattackstate "NewEnumerator2")
  (bind _outhit (Collision|LineTraceForObjects _returnvalue (+ _returnvalue (* (Transformation|GetActorForwardVector) 1.5e+02)) (Utilities|Array|MakeArray "ObjectTypeQuery3") false (Utilities|Array|MakeArray self) "None"))
  (if (== (.HitActor (Collision|BreakHitResult _outhit)) (Game|GetPlayerCharacter 0))
    (Game|Damage|ApplyDamage (.HitActor (Collision|BreakHitResult _outhit)) (Variables|Edit|Getenemydamage) 0 0))
  (Utilities|FlowControl|RetriggerableDelay (+ (Variables|Edit|GetMeleerate) 0.1))
  (Variables|Donotedit|Setisattacking false))

(event Custom|Handle%20death
  (bind _paperflipbook (Variables|Default|GetPaperFlipbook))
  ;[1 1 1] Handle enemy death system
  (Transformation|SetActorRotation (Math|Rotator|MakeRotator 0.0 0.0 (.yaw (Math|Rotator|FindLookatRotation (Transformation|GetActorLocation) (Transformation|GetActorLocation (Game|GetPlayerCharacter 0))))))
  (Utilities|FlowControl|DoOnce false
    (:Completed
      (AI|Logic|StopLogic (Variables|/Script/AIModule.AIController|GetBrainComponent (AI|GetAIController self)) "isdead")
      (Pawn|Components|CharacterMovement|SetMovementMode (Variables|Character|GetCharacterMovement) "MOVE_Flying" 0)
      (Collision|SetCollisionEnabled (Variables|Collision|GetCapsuleComponent) "NoCollision")
      (Components|Activation|Deactivate (Variables|Character|GetCharacterMovement))
      (Transformation|SetRelativeRotation _paperflipbook "0.000000,-90.000000,0.000000" false false)
      (Sprite|SetFlipbook _paperflipbook (Variables|Flipbooks|Getenemydeathflipbook))
      (Utilities|FlowControl|Delay (- (Class|PaperFlipbookComponent|GetFlipbookLength (Variables|Default|GetPaperFlipbook)) 0.2))
      (Transformation|AddActorLocalOffset "0.000000,0.000000,-30.000000" false false)
      (Sprite|SetFlipbook (Variables|Default|GetPaperFlipbook) (Variables|Flipbooks|Getenemybodyflipbook))
      (Utilities|FlowControl|Delay 4.0)
      (Actor|DestroyActor))))

(event EventTick
  (params (DeltaSeconds :type Float%20%28single-precision%29))
  (bind _returnvalue (|handleenemystate+calcuateenemydegrees))
  (|setenemyrotation+flipbook _returnvalue))

(event Game|Damage|EventAnyDamage
  (params (Damage :type Float%20%28single-precision%29) (DamageType :type Damage%20Type%20Object%20Reference) (InstigatedBy :type Controller%20Object%20Reference) (DamageCauser :type Actor%20Object%20Reference))
  ;[1 1 1] handle enemy damage
  (bind _output_get (Variables|Edit|Sethealth (- (Variables|Edit|Gethealth) Damage)))
  (if (<= _output_get 0.0)
    (Variables|Donotedit|Setisdead true)
    (else
      (Variables|donotedit|Setcanseeplayer true)
      (AI|Components|Blackboard|SetValueasBool (AI|GetBlackboard 0) (Utilities|Name|MakeLiteralName "canseeplayer") true))))

(fn ConstructionScript)